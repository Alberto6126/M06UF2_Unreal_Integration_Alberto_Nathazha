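; BP_ZoneAudioCueva is an audio zone, named for a cave, that plays a configurable sound while the player character is inside it.
; On BeginPlay it assigns SoundPick to the ZoneSound component and fades it in immediately if IsSpawn is set.
; Actor overlaps with BP_ThirdPersonCharacter fade the sound in on entry and out on exit, with debug prints left on the fade-ins.
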(event EventBeginPlay
  (Audio|Components|Audio|SetSound (Variables|Default|GetZoneSound) (Variables|Default|GetSoundPick))
  (if (Variables|Default|GetisSpawn)
    (Audio|Components|Audio|FadeIn (Variables|Default|GetZoneSound) (Variables|Default|GetinitialFade) 1.0 0.0 "Linear" :!class /Script/Engine.AudioComponent)
    (Development|PrintString "Hello")))

(event Collision|EventActorBeginOverlap
  (params (OtherActor :type Actor%20Object%20Reference))
  (Utilities|Casting|CastToBP_ThirdPersonCharacter OtherActor)
  (Audio|Components|Audio|FadeIn (Variables|Default|GetZoneSound) (Variables|Default|GetFadeDuration) 1.0 0.0 "Linear" :!class /Script/Engine.AudioComponent)
  (Development|PrintString "Hello"))

(event Collision|EventActorEndOverlap
  (params (OtherActor :type Actor%20Object%20Reference))
  (Utilities|Casting|CastToBP_ThirdPersonCharacter OtherActor)
  (Audio|Components|Audio|FadeOut (Variables|Default|GetZoneSound) (Variables|Default|GetFadeDuration) 0.0 "Linear" :!class /Script/Engine.AudioComponent))

(fn ConstructionScript)