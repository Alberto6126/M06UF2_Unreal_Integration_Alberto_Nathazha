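; Projectile actor that flies in a straight line and explodes when destroyed.
; Each Tick calls ProjectileMovement, which offsets the root component by Direction, Speed and Sense scaled by delta time, teleporting without a sweep.
; On Destroyed it spawns an explosion particle effect and sound at its location.
; The file contains no collision or destruction trigger of its own.
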(event EventTick
  (params (DeltaSeconds :type Float%20%28single-precision%29))
  (Utilities|ProjectileMovement DeltaSeconds))

(event EventDestroyed
  (bind _returnvalue (Transformation|GetActorLocation))
  ;[1 1 1] Al destruirse el proyectil se spawnean partículas y sonido
  (Effects|SpawnEmitteratLocation "/Game/CORREGIR/Particles/P_Explosion.P_Explosion" _returnvalue)
  (Audio|SpawnSoundatLocation "/Game/CORREGIR/Audio/Sounds/Cues/Explosions.Explosions" _returnvalue "0, 0, 0" 1.0 1.0 0.0 0 0))

(fn ConstructionScript)