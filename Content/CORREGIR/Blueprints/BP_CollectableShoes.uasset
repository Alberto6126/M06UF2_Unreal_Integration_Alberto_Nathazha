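; BP_CollectableShoes is a pickup actor that turns on the boots state of the BP_ThirdPersonCharacter that overlaps it.
; On overlap, ActivateShoes calls SetBootsOn on the character and hides both shoe components, then the actor plays two collection sounds separated by a short delay and destroys itself.
; Tick spins the actor around its local yaw axis through RotateObject, scaled by delta time, speed and direction.
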(event Collision|EventActorBeginOverlap
  (params (OtherActor :type Actor%20Object%20Reference))
  (bind _asbp_third_person_character (Utilities|Casting|CastToBP_ThirdPersonCharacter OtherActor))
  (Utilities|ActivateShoes _asbp_third_person_character
    (:Out
      (Audio|SpawnSound2D "/Game/CORREGIR/Audio/Sounds/Waves/SFX/ItemCollected_2.ItemCollected_2" 1.0 1.0 0.0 0)
      (Utilities|FlowControl|Delay 0.5)
      (Audio|SpawnSound2D "/Game/CORREGIR/Audio/Sounds/Waves/SFX/ItemCollected_1.ItemCollected_1" 1.0 1.0 0.0 0)
      (Actor|DestroyActor))))

(event EventTick
  (params (DeltaSeconds :type Float%20%28single-precision%29))
  (Utilities|RotateObject DeltaSeconds))

(fn ConstructionScript)